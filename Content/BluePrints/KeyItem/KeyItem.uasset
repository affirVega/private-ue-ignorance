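; KeyItem is an actor that detects when it is on screen and pulls the player's view to itself.
; Every tick it projects its location to screen space for player 0, checks it against the viewport bounds, sets OnScreen and prints a debug YES or NO.
; While on screen, it calls a cubic view-target blend to itself every tick.
; The visibility test has no occlusion trace.
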(event `self.ReceiveTick`
  (params (DeltaSeconds :type "Float (single-precision)"))
  (bind (_returnvalue_x _returnvalue_y) (`KismetMathLibrary.BreakVector2D` (`WidgetLayoutLibrary.GetViewportSize`)))
  (bind _screenlocation (`PlayerController.ProjectWorldLocationToScreen` (`GameplayStatics.GetPlayerController` 0) (`self.K2_GetActorLocation`) false))
  (if (and (> (`KismetMathLibrary.BreakVector2D` _screenlocation) 0.0) (> (`.Y` (`KismetMathLibrary.BreakVector2D` _screenlocation)) 0.0) (< (`KismetMathLibrary.BreakVector2D` _screenlocation) _returnvalue_x) (< (`.Y` (`KismetMathLibrary.BreakVector2D` _screenlocation)) _returnvalue_y))
    (`KismetSystemLibrary.PrintString` "YES" true true (struct :`G` 0.66 :`B` 1.0 :`A` 1.0) 0.01)
    (set `self.OnScreen` true)
    (`PlayerController.SetViewTargetWithBlend` (`GameplayStatics.GetPlayerController` 0) self 1.0 "VTBlend_Cubic" 0.0 false)
    (else
      (`KismetSystemLibrary.PrintString` "NO" true true (struct :`G` 0.66 :`B` 1.0 :`A` 1.0) 0.01)
      (set `self.OnScreen` false))))

(fn `UserConstructionScript`)