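; RangeTarget_BP is a moving target dummy that reacts to projectile hits.
; On BeginPlay, two timelines lerp it back and forth between its starting location and a fixed Y coordinate, restarting each other in an endless loop.
; A Projectile overlapping its box plays a one-shot back-shot animation on the skeletal mesh, with no damage or scoring.
; It caches a player reference that goes unused, though movement only starts if that cast succeeds.
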(event `self.ReceiveBeginPlay`
  (bind (_returnvalue_x _returnvalue_y _returnvalue_z) (`KismetMathLibrary.BreakVector` (`self.K2_GetActorLocation`)))
  (set `self.Start` (`KismetMathLibrary.MakeVector` _returnvalue_x _returnvalue_y _returnvalue_z))
  (set `self.End` (`KismetMathLibrary.MakeVector` _returnvalue_x 2000.0 _returnvalue_z))
  (bind _asbp_player_base (cast `/Game/BluePrints/Player_Camera/BP_PlayerBase` (`GameplayStatics.GetPlayerCharacter` 0)))
  (set `self.Player ref` _asbp_player_base)
  (bind (_direction _move) (`Timeline|Move` :!via `PlayFromStart` :!label _label)
    (:`Update`
      (`self.K2_SetActorRelativeLocation` (`KismetMathLibrary.VLerp` (`self.Start`) (`self.End`) _move)))
    (:`Finished`
      (bind (_direction_2 _move_2) (`Timeline|MoveBack` :!via `ReverseFromEnd`)
        (:`Update`
          (`self.K2_SetActorRelativeLocation` (`KismetMathLibrary.VLerp` (`self.Start`) (`self.End`) _move_2)))
        (:`Finished`
          (goto _label :!via `PlayFromStart`))))))

(event `self.Box.OnComponentBeginOverlap`
  (params (OverlappedComponent :type "PrimitiveComponent Object Reference") (OtherActor :type "Actor Object Reference") (OtherComp :type "PrimitiveComponent Object Reference") (OtherBodyIndex :type Integer) (bFromSweep :type Boolean) (SweepResult :type "HitResult Structure (by ref)"))
  (cast `/Game/BluePrints/Player_Camera/Shooting/Projectile` OtherActor)
  (`SkeletalMeshComponent.PlayAnimation` (`self.SkeletalMesh`) "/Game/BluePrints/Player_Camera/Dummy/Dummy_Anim__1__Cube_Anim_Dummy_BackShot.Dummy_Anim__1__Cube_Anim_Dummy_BackShot" false))

(fn `UserConstructionScript`)