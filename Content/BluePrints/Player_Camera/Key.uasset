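; Key actor in the player camera folder that shifts its own Camera component toward the player while it is on screen and nearby.
; Each tick it projects its location to screen space, checks viewport bounds and player distance, and sets the Seen flag.
; While seen, the camera's starting relative location is offset by the key-to-player vector divided by FloatTwo.
; When unseen, only the flag clears; the camera stays put.
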(event `self.ReceiveBeginPlay`
  (set `self.CameraPosition` (`SceneComponent.RelativeLocation` (`self.Camera`))))

(event `self.ReceiveTick`
  (params (DeltaSeconds :type "Float (single-precision)"))
  (bind (_returnvalue_x _returnvalue_y) (`KismetMathLibrary.BreakVector2D` (`WidgetLayoutLibrary.GetViewportSize`)))
  (bind _screenlocation (`PlayerController.ProjectWorldLocationToScreen` (`GameplayStatics.GetPlayerController` 0) (`self.K2_GetActorLocation`) false))
  (bind _returnvalue (- (`self.K2_GetActorLocation` (`GameplayStatics.GetPlayerCharacter` 0)) (`self.K2_GetActorLocation` self)))
  (`/Engine/EditorBlueprintResources/StandardMacros.IsValid` (`GameplayStatics.GetPlayerCharacter` 0)
    (:`Is Valid`
      (if (and (> (`KismetMathLibrary.BreakVector2D` _screenlocation) 0.0) (> (`.Y` (`KismetMathLibrary.BreakVector2D` _screenlocation)) 0.0) (< (`KismetMathLibrary.BreakVector2D` _screenlocation) _returnvalue_x) (< (`.Y` (`KismetMathLibrary.BreakVector2D` _screenlocation)) _returnvalue_y) (< (`KismetMathLibrary.VSize` _returnvalue) 670.0))
        (set `self.Seen` true)
        (`SceneComponent.K2_SetRelativeLocation` (`self.Camera`) (+ (`self.CameraPosition`) (/ _returnvalue (`self.FloatTwo`))) false false)
        (else
          (set `self.Seen` false))))))

(fn `UserConstructionScript`)