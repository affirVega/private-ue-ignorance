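; BP_PatrpolPath is a patrol path actor that holds a list of PathPoints.
; GetPoint converts an indexed point from local to world space by applying the root component's rotation, scale and location, with scale multiplied after rotation.
; GetLength returns the number of points rather than a distance, and the construction script is empty.
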(fn `GetLength`
  (returns (Length :type Integer))
  (return (`KismetArrayLibrary.Array_Length` (`self.PathPoints`))))

(fn `GetPoint`
  (params (Index :type Integer))
  (returns (Vector :type "Vector Structure"))
  (bind _defaultsceneroot (`self.DefaultSceneRoot`))
  (return (+ (* (`KismetMathLibrary.GreaterGreater_VectorRotator` (`|GetArrayItem` (`self.PathPoints`) Index) (`SceneComponent.K2_GetComponentRotation` _defaultsceneroot)) (`SceneComponent.K2_GetComponentScale` _defaultsceneroot)) (`SceneComponent.K2_GetComponentLocation` _defaultsceneroot))))

(fn `UserConstructionScript`)