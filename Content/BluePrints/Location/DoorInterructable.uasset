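; DoorInterructable is a door Blueprint that raises and lowers its Sphere component along relative Z.
; OpenDoor stores a target Height and derives Speed from TimeToOpen; CloseDoor resets the target to zero only when ShouldClose is set, reusing that speed.
; Tick moves the Sphere toward the target at constant speed with FInterpToConstant.
; The IsClosed flag reads inverted: it becomes true on opening and blocks repeated opens.
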(event `OpenDoor`
  (params (Height :type "Float (double-precision)" :default 300.0) (TimeToOpen :type "Float (double-precision)" :default 1.0))
  ;[1 1 1] Выполнение кода открывания двери должно срабатывать когда дверь была закрыта и она открывается.
  (`self.FOpenDoor` Height TimeToOpen))

(event `CloseDoor`
  ;[1 1 1] Выполнение кода открывания двери должно срабатывать когда дверь была закрыта и она открывается.
  (`self.FCloseDoor`))

(event `self.ReceiveTick`
  (params (DeltaSeconds :type "Float (single-precision)"))
  (bind _sphere (`self.Sphere`))
  (bind (_relativelocation_x _relativelocation_y _relativelocation_z) (`KismetMathLibrary.BreakVector` (`SceneComponent.RelativeLocation` (`self.Sphere`))))
  (bind (_relativelocation_x_2 _relativelocation_y_2) (`KismetMathLibrary.BreakVector` (`SceneComponent.RelativeLocation` _sphere)))
  (`SceneComponent.K2_SetRelativeLocation` _sphere (`KismetMathLibrary.MakeVector` _relativelocation_x_2 _relativelocation_y_2 (`KismetMathLibrary.FInterpTo_Constant` _relativelocation_z (`self.Height`) DeltaSeconds (`self.Speed`))) false false))

(fn `FCloseDoor`
  (if (`self.ShouldClose`)
    (set `self.IsClosed` false)
    (set `self.Height` 0.0)))

(fn `FOpenDoor`
  (params (Height :type "Float (double-precision)" :default 200.0) (TimeToOpen :type "Float (double-precision)" :default 1.0))
  (if (not (`self.IsClosed`))
    (set `self.Height` Height)
    (set `self.IsClosed` true)
    (set `self.Speed` (/ Height TimeToOpen))))

(fn `UserConstructionScript`)