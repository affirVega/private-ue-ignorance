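; ButtonOpen is a door button actor that opens a linked door when the player presses E nearby.
; Overlap events on its Trigger enable the actor's input when a BP_PlayerBase enters and disable it on exit, using player controller 0.
; A DoOnce lets the key press call OpenDoor on DoorRef only once.
; BeginPlay prints a red warning with the button's location if DoorRef is unset.
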(event `self.ReceiveBeginPlay`
  (`/Engine/EditorBlueprintResources/StandardMacros.IsValid` (`self.DoorRef`)
    (:`Is Not Valid`
      (`KismetSystemLibrary.PrintText` (`|FormatText` "Button <ButtonOpen {xyz}> has no Door reference. Please set it manually" (`KismetStringLibrary.Conv_VectorToString` (`SceneComponent.K2_GetComponentLocation` (`self.DefaultSceneRoot`)))) true true (struct :`R` 1.0 :`B` 0.040099 :`A` 1.0) 20.0))))

(event `self.Trigger.OnComponentBeginOverlap`
  (params (OverlappedComponent :type "PrimitiveComponent Object Reference") (OtherActor :type "Actor Object Reference") (OtherComp :type "PrimitiveComponent Object Reference") (OtherBodyIndex :type Integer) (bFromSweep :type Boolean) (SweepResult :type "HitResult Structure (by ref)"))
  (cast `/Game/BluePrints/Player_Camera/BP_PlayerBase` OtherActor)
  (`self.EnableInput` (`GameplayStatics.GetPlayerController` 0)))

(event `self.Trigger.OnComponentEndOverlap`
  (params (OverlappedComponent :type "PrimitiveComponent Object Reference") (OtherActor :type "Actor Object Reference") (OtherComp :type "PrimitiveComponent Object Reference") (OtherBodyIndex :type Integer))
  (cast `/Game/BluePrints/Player_Camera/BP_PlayerBase` OtherActor)
  (`self.DisableInput` (`GameplayStatics.GetPlayerController` 0)))

(event `Key|E`
  (params (Key :type "Key Structure"))
  (:`Pressed`
    (`/Engine/EditorBlueprintResources/StandardMacros.DoOnce` false
      (:`Completed`
        (`/Game/BluePrints/Location/DoorInterructable.OpenDoor` (`self.DoorRef`))))))

(fn `UserConstructionScript`)