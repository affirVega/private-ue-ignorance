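; GameManager actor that shows a one-time tutorial hint for opening doors.
; ShowTutorialOpenDoor passes a DoOnce, creates the DoorOpen widget as HintUI and adds it to the viewport.
; The CanvasTransparency timeline drives the canvas opacity, with a FlipFlop on Finished reversing the fade, then removing the widget.
; A trailing three-second Delay leads to nothing, so it does not hold the hint on screen.
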(event `self.ReceiveBeginPlay`)

(event `ShowTutorialOpenDoor`
  (`/Engine/EditorBlueprintResources/StandardMacros.DoOnce` false
    (:`Completed`
      (bind _returnvalue (`|CreateWidget` "/Game/BluePrints/Location/DoorOpen.DoorOpen_C"))
      (set `self.HintUI` _returnvalue)
      (`|ExecutionSequence`
        (:`then_0`
          (bind (_direction _opacity) (`Timeline|CanvasTransparency` :!label _label)
            (:`Update`
              (`Widget.SetRenderOpacity` (`/Game/BluePrints/Location/DoorOpen.Canvas_1` (`self.HintUI`)) _opacity))
            (:`Finished`
              (`/Engine/EditorBlueprintResources/StandardMacros.FlipFlop`
                (:`A`
                  (goto _label :!via `Reverse`))
                (:`B`
                  (`Widget.RemoveFromParent` (`self.HintUI`)))))))
        (:`then_1`
          (`UserWidget.AddToViewport` (`self.HintUI`) 0)
          (`KismetSystemLibrary.Delay` 3.0))))))

(fn `UserConstructionScript`)