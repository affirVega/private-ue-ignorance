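; Behavior tree task that advances an enemy to the next point on its patrol path.
; It casts the controlled pawn to BP_Enemy and reads the length of its PatrolPath.
; It increments the path index stored in the blackboard, wrapping to zero at the end so the patrol loops, then finishes with success.
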(event `self.ReceiveExecuteAI`
  (params (OwnerController :type "AIController Object Reference") (ControlledPawn :type "Pawn Object Reference"))
  (bind _bb_pathindex (`self.BB_PathIndex`))
  (bind _returnvalue (+ (`BTFunctionLibrary.GetBlackboardValueAsInt` (`self.BB_PathIndex`)) 1))
  (bind _asbp_enemy (cast `/Game/BluePrints/Enemy/BP_Enemy` ControlledPawn))
  (bind _length (`/Game/BluePrints/Spline/BP_PatrpolPath.GetLength` (`/Game/BluePrints/Enemy/BP_Enemy.PatrolPath` _asbp_enemy)))
  (if (< _returnvalue _length)
    (`BTFunctionLibrary.SetBlackboardValueAsInt` _bb_pathindex _returnvalue)
    (else
      (`BTFunctionLibrary.SetBlackboardValueAsInt` _bb_pathindex)))
  (`self.FinishExecute` true))